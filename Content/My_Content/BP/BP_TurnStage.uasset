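; BP_TurnStage is a stage-turning actor whose box overlap alternately turns the player ThirdPersonCharacter's camera left and right.
; A timeline event spins each listed actor and orbits it around Centre by a fixed angle per update along the chosen X/Y axis, then resets the axis and re-arms the switch.
; The four direction branches that set the axis and start this rotation have no triggers, so they never run.
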(event `self.Box.OnComponentBeginOverlap`
  (params (OverlappedComponent :type "PrimitiveComponent Object Reference") (OtherActor :type "Actor Object Reference") (OtherComp :type "PrimitiveComponent Object Reference") (OtherBodyIndex :type Integer) (bFromSweep :type Boolean) (SweepResult :type "HitResult Structure (by ref)"))
  (`KismetSystemLibrary.PrintString` "Hello")
  (`/Engine/EditorBlueprintResources/StandardMacros.FlipFlop`
    (:`A`
      (bind _asthird_person_character (cast `/Game/ThirdPersonBP/Blueprints/ThirdPersonCharacter` (`GameplayStatics.GetPlayerCharacter` 0)))
      (`/Game/ThirdPersonBP/Blueprints/ThirdPersonCharacter.TurnCameraLeft` _asthird_person_character))
    (:`B`
      (bind _asthird_person_character_2 (cast `/Game/ThirdPersonBP/Blueprints/ThirdPersonCharacter` (`GameplayStatics.GetPlayerCharacter` 0)))
      (`/Game/ThirdPersonBP/Blueprints/ThirdPersonCharacter.TurnCameraRight` _asthird_person_character_2))))

(event `カスタムイベント_0`
  (bind _returnvalue (`self.K2_GetActorLocation` (`self.centre`)))
  (bind _asthird_person_character (cast `/Game/ThirdPersonBP/Blueprints/ThirdPersonCharacter` (`GameplayStatics.GetPlayerCharacter` 0)))
  (set `/Game/ThirdPersonBP/Blueprints/ThirdPersonCharacter.111` 30.0 _asthird_person_character)
  (`Timeline|タイムライン_0` :!label _label ; 不要动这个。。。
    (:`Update`
      (for _array_element (`self.Actor`)
        (if (`KismetSystemLibrary.IsValid` (break `/Game/My_Content/BP/BP_SceneInfo` _array_element))
          (`SceneComponent.K2_AddWorldRotation` (`Actor.RootComponent` (break `/Game/My_Content/BP/BP_SceneInfo` _array_element)) (`self.Delta Rotation`) false false)
          (`self.K2_SetActorLocation` (break `/Game/My_Content/BP/BP_SceneInfo` _array_element) (+ (`KismetMathLibrary.RotateAngleAxis` (- (`self.K2_GetActorLocation` (break `/Game/My_Content/BP/BP_SceneInfo` _array_element)) _returnvalue) 1.475 (`KismetMathLibrary.MakeVector` (`self.X`) (`self.Y`))) _returnvalue) false false))))
    (:`Finished`
      (`self.カスタムイベント_1`)
      (goto _label :!via `SetNewTime`))))

(event `カスタムイベント_1`
  (set `self.X` 0.0)
  (set `self.Y` 0.0)
  (set `self.Delta Rotation` (struct))
  (set `self.Swich` true))

(fn `UserConstructionScript`)