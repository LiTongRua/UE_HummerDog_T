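; BP_Roll is an actor that rotates an array of actors around a Centre actor when number keys 1 to 4 are pressed.
; Each key sets an axis component, never clearing the other, and a delta rotation, then plays the shared 回転 (rotation) timeline.
; Timeline updates spin each actor's root and swing its current location around Centre by the track's angle.
; Tick re-enables input every frame, and the timeline resets its time on finish.
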(event `self.ReceiveTick`
  (params (DeltaSeconds :type "Float (single-precision)"))
  (`self.EnableInput` (`GameplayStatics.GetPlayerController` 0)))

(event `Key|One`
  (params (Key :type "Key Structure"))
  (bind _returnvalue (`self.K2_GetActorLocation` (`self.centre`)))
  (:`Pressed`
    (set `self.X` 1.0)
    (set `self.Delta Rotation` (struct :`Roll` 1.475))
    (bind (_direction `_回転`) (`Timeline|回転` :!label _label)
      (:`Update`
        (for _array_element (`self.Actor`)
          (`SceneComponent.K2_AddRelativeRotation` (`Actor.RootComponent` (break `/Game/My_Content/BP/BP_SceneInfo` _array_element)) (`self.Delta Rotation`) false false)
          (`self.K2_SetActorLocation` (break `/Game/My_Content/BP/BP_SceneInfo` _array_element) (+ (`KismetMathLibrary.RotateAngleAxis` (- (`self.K2_GetActorLocation` (break `/Game/My_Content/BP/BP_SceneInfo` _array_element)) _returnvalue) `_回転` (`KismetMathLibrary.MakeVector` (`self.X`) (`self.Y`) (`self.Z`))) _returnvalue) false false)))
      (:`Finished`
        (if true
          (goto _label :!via `SetNewTime`))))))

(event `Key|Two`
  (params (Key :type "Key Structure"))
  (:`Pressed`
    (set `self.Z` 1.0)
    (set `self.Delta Rotation` (struct :`Yaw` 1.475))
    (goto _label)))

(event `Key|Three`
  (params (Key :type "Key Structure"))
  (:`Pressed`
    (set `self.X` -1.0)
    (set `self.Delta Rotation` (struct :`Pitch` -1.475))
    (goto _label)))

(event `Key|Four`
  (params (Key :type "Key Structure"))
  (:`Pressed`
    (set `self.Z` -1.0)
    (set `self.Delta Rotation` (struct :`Yaw` -1.475))
    (goto _label)))

(fn `UserConstructionScript`)