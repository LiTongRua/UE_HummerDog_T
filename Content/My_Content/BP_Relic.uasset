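; BP_Relic is a relic actor that shows a warning when an actor tagged "dog" comes near it.
; Beginning an overlap with its Warning component plays the SD_GetStar_Cue sound at that component's location and makes SMWarning visible.
; Ending the overlap hides SMWarning again.
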(event `self.Warning.OnComponentBeginOverlap`
  (params (OverlappedComponent :type "PrimitiveComponent Object Reference") (OtherActor :type "Actor Object Reference") (OtherComp :type "PrimitiveComponent Object Reference") (OtherBodyIndex :type Integer) (bFromSweep :type Boolean) (SweepResult :type "HitResult Structure (by ref)"))
  (if (`self.ActorHasTag` OtherActor "dog")
    (`GameplayStatics.PlaySoundAtLocation` "/Game/My_Content/SD/SD_GetStar_Cue.SD_GetStar_Cue" (`SceneComponent.K2_GetComponentLocation` OverlappedComponent) (struct) 1.0 1.0 0.0 null null null)
    (`SceneComponent.SetVisibility` (`self.SM_Warning`) true false)))

(event `self.Warning.OnComponentEndOverlap`
  (params (OverlappedComponent :type "PrimitiveComponent Object Reference") (OtherActor :type "Actor Object Reference") (OtherComp :type "PrimitiveComponent Object Reference") (OtherBodyIndex :type Integer))
  (if (`self.ActorHasTag` OtherActor "dog")
    (`SceneComponent.SetVisibility` (`self.SM_Warning`) false false)))

(fn `UserConstructionScript`)